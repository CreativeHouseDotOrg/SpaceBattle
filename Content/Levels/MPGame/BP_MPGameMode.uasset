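; BP_MPGameMode is the game mode for a multiplayer level, registering players as they log in.
; PostLogin adds each BP_MPPlayerController to PlayerControllerList and prints a success message with the player's name.
; ReadyToStartMatch always returns true, leaving its player-count check unused.
; A disconnected branch would call MatchStartedEvent on BP_MPGameState once the player count equals MaxPlayers, but it never runs.
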(event `self.K2_PostLogin`
  (params (NewPlayer :type "PlayerController Object Reference"))
  (`self.AddPlayerController` NewPlayer))

(fn `AddPlayerController`
  (params (PlayerController :type "Object Object Reference"))
  (bind _asbp_player_controller (cast `/Game/Levels/MPGame/BP_MPPlayerController` PlayerController))
  (`KismetArrayLibrary.Array_Add` (`self.PlayerControllerList`) _asbp_player_controller)
  (`/Game/Libraries/PrintLib.PrintSuccess` (`self.PrintLib`) (`KismetStringLibrary.Concat_StrStr` "added " (`PlayerState.GetPlayerName` (`Controller.PlayerState` _asbp_player_controller)) " to PlayerList!") 20.0))

(fn `FN_GetGameState`
  (returns (GameState :type "/Game/Levels/MPGame/BP_MPGameState Object Reference"))
  (bind _asbp_game_state (cast `/Game/Levels/MPGame/BP_MPGameState` (`GameplayStatics.GetGameState`)))
  (return _asbp_game_state))

(fn `ReadyToStartMatch`
  (returns (ReturnValue :type Boolean))
  (return true))

(fn `UserConstructionScript`)