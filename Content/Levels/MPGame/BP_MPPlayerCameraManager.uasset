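; Camera manager for the multiplayer game that keeps a list of cameras and controls screen fades.
; Events register new cameras and destroy stray default CameraActors, found by a name substring match.
; Fades use manual camera fade on player 0: a solid black fill, plus a white fade timeline played or reversed at a duration-based rate.
; An active-camera getter wraps an index-lookup macro, while first-camera initialization is an empty stub.
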(event `AddCameraEvent`
  (params (NewCamera :type "/Game/Levels/MPGame/BP_MPGameCamera Object Reference"))
  (`self.FN_AddCamera` NewCamera))

(event `InitFirstCameraEvent`)

(event `DestroyDefaultCameraEvent`
  ;[1 0 0] Destroy strange default camera that gets spawned from Hell
  (`self.FN_DestroyDefaultCamera`))

(event `FillScreenWithSolidColorEvent`
  ;[0 0 0] Fill the screen with a solid color when the game starts
  (`self.SetManualCameraFade` (`GameplayStatics.GetPlayerCameraManager` 0) 1.0 (struct :`A` 1.0) false))

(event `FadeInOutEvent`
  (params (SecondsToFade :type "Float (double-precision)") (bFadeIn :type Boolean))
  ;[0 0 0] How many Seconds does it take to fade?
  (`TimelineComponent.SetPlayRate` (`self.TL_CameraFadeInOut`) (/ 1.0 SecondsToFade))
  ;[0 0 0] Fade in or out?
  (if bFadeIn
    ;[0 0 0] Perform the Fading
    (bind (_direction _fadeamount) (`Timeline|TL_CameraFadeInOut` :!label _label)
      (:`Update`
        (`self.SetManualCameraFade` (`GameplayStatics.GetPlayerCameraManager` 0) _fadeamount (struct :`R` 1.0 :`G` 1.0 :`B` 1.0 :`A` 1.0) false)))
    (else
      (goto _label :!via `Reverse`))))

(fn `FN_AddCamera`
  (params (NewCamera :type "/Game/Levels/MPGame/BP_MPGameCamera Object Reference"))
  (`KismetArrayLibrary.Array_Add` (`self.Cameras`) NewCamera)
  (return))

(fn `FN_DestroyDefaultCamera`
  (bind _outactors (`GameplayStatics.GetAllActorsOfClass` "/Script/Engine.CameraActor"))
  (for _array_element _outactors
    (if (`KismetStringLibrary.Contains` (`KismetSystemLibrary.GetObjectName` _array_element) "CameraActor")
      (`self.K2_DestroyActor` _array_element))))

(fn `FN_GetActiveCamera`
  (returns (ActiveCamera :type "/Game/Levels/MPGame/BP_MPGameCamera Object Reference"))
  (return (`self.M_GetActiveCamera`)))

(fn `UserConstructionScript`)