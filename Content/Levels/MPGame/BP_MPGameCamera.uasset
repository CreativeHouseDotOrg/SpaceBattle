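; BP_MPGameCamera is the multiplayer level's camera actor, which registers itself with the player's BP_MPPlayerCameraManager.
; BeginPlay and the InitCamera event both run FNInitCamera, which passes the camera to the manager's AddCameraEvent on clients only and prints a warning on authority.
; A separate event resets the actor to a hard-coded elevated default transform through small location and rotation setter functions.
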(event `self.ReceiveBeginPlay`
  (`self.FN_InitCamera` :!label _label))

(event `InitCamera`
  (goto _label))

(event `SetDefaultCameraTransformEvent`
  (`self.FN_SetDefaultTransform`))

(fn `FN_GetPlayerCameraManager`
  (returns (CameraManager :type "/Game/Levels/MPGame/BP_MPPlayerCameraManager Object Reference"))
  (bind _asbp_mpplayer_camera_manager (cast `/Game/Levels/MPGame/BP_MPPlayerCameraManager` (`GameplayStatics.GetPlayerCameraManager` 0)))
  (return _asbp_mpplayer_camera_manager))

(fn `FN_InitCamera`
  (bind _cameramanager (`self.FN_GetPlayerCameraManager`))
  (`/Engine/EditorBlueprintResources/ActorMacros.Switch Has Authority`
    (:`Authority`
      (`/Game/Libraries/FL_PrintLib.PrintWarning` "CameraManager can not be set on Server"))
    (:`Remote`
      (`/Game/Levels/MPGame/BP_MPPlayerCameraManager.AddCameraEvent` _cameramanager self))))

(fn `FN_SetCameraLocation`
  (params (Location :type "Vector Structure"))
  (`self.K2_SetActorLocation` Location)
  (return))

(fn `FN_SetCameraRotation`
  (params (Rotation :type "Rotator Structure"))
  (`self.K2_SetActorRotation` Rotation)
  (return))

(fn `FN_SetDefaultTransform`
  (`|ExecutionSequence`
    (:`then_0`
      (`self.FN_SetCameraLocation` (0.0 0.0 500.0)))
    (:`then_1`
      (`self.FN_SetCameraRotation` (struct :`Pitch` -90.0)))))

(fn `UserConstructionScript`)