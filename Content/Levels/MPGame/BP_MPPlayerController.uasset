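; Multiplayer player controller that handles client-side camera startup and mouse activation.
; BeginPlay activates the mouse and asks BP_MPPlayerCameraManager to initialize the first camera.
; ClientInitialize fills the screen with a solid color, reactivates the mouse, resets the active camera to its default transform, then fades in.
; Camera work is delegated to the camera manager through small wrapper functions, with an error printed when no active camera exists.
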(event `self.ReceiveBeginPlay`
  (`/Game/Libraries/FL_MouseLib.FN_ActivateMouse`)
  (`self.FN_InitCamera`))

(event `ClientInitialize`
  (`|ExecutionSequence`
    (:`then_0`
      (bind _cameramanager (`self.FN_GetPlayerCameraManager`))
      (`/Game/Levels/MPGame/BP_MPPlayerCameraManager.FillScreenWithSolidColorEvent` _cameramanager))
    (:`then_1`
      (`/Game/Libraries/FL_MouseLib.FN_ActivateMouse`))
    (:`then_2`
      (`self.FN_CameraSetDefaultTransform`))
    (:`then_3`
      (`self.FN_FadeCamera` true))))

(fn `FN_CameraSetDefaultTransform`
  (bind _cameramanager (`self.FN_GetPlayerCameraManager`))
  (bind _activecamera (`/Game/Levels/MPGame/BP_MPPlayerCameraManager.FN_GetActiveCamera` _cameramanager))
  (`/Engine/EditorBlueprintResources/StandardMacros.IsValid` _activecamera
    (:`Is Valid`
      (`/Game/Levels/MPGame/BP_MPGameCamera.SetDefaultCameraTransformEvent` _activecamera)
      (return))
    (:`Is Not Valid`
      (`/Game/Libraries/FL_PrintLib.PrintError` "No Active Camera set!"))))

(fn `FN_FadeCamera`
  (params (bFadeIn :type Boolean))
  (bind _cameramanager (`self.FN_GetPlayerCameraManager`))
  (`/Game/Levels/MPGame/BP_MPPlayerCameraManager.FadeInOutEvent` _cameramanager 2.0 bFadeIn)
  (return))

(fn `FN_GetPlayerCameraManager`
  (returns (CameraManager :type "/Game/Levels/MPGame/BP_MPPlayerCameraManager Object Reference"))
  (bind _asbp_mpplayer_camera_manager (cast `/Game/Levels/MPGame/BP_MPPlayerCameraManager` (`GameplayStatics.GetPlayerCameraManager` 0)))
  (return _asbp_mpplayer_camera_manager))

(fn `FN_InitCamera`
  (bind _cameramanager (`self.FN_GetPlayerCameraManager`))
  (`/Game/Levels/MPGame/BP_MPPlayerCameraManager.InitFirstCameraEvent` _cameramanager))

(fn `UserConstructionScript`)