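; BP_Ship is an AI-controlled ship unit holding health, shield and energy stats plus attack and regeneration values, which a reset event restores to fixed defaults.
; On BeginPlay it passes its radius to the ACCircle component, and an event shows or hides its ShipStats widget.
; Movement sends a stored target location to the custom AI controller's MoveToTargetEvent, with unused Blackboard and MoveToLocation alternatives left unconnected.
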(event `self.ReceiveBeginPlay`
  (`self.ChangeShipRadius` (`self.ShipRadius`)))

(event `ChangeShipRadius`
  (params (Radius :type "Float (double-precision)"))
  (set `self.ShipRadius` Radius)
  (`/Game/Levels/Game/Circle/AC_Circle.ChangeRadiusEvent` (`self.AC_Circle`) (`self.ShipRadius`)))

(event `ToggleShipStats`
  (params (Show :type Boolean))
  (`SceneComponent.SetHiddenInGame` (`self.ShipStats`) (not Show) false))

(event `ResetValuesEvent`
  (`self.FN_ResetValues`))

(fn `FN_MoveToTargetLocation`
  (returns (TargetLocation :type "Vector Structure"))
  ;[0 0 0] Move via custom "MoveToTargetEvent" inside of our own AIC_AI Controller Class
  (`/Game/Levels/Game/Controllers/AI/AIC_AI.MoveToTargetEvent` (`/Game/Levels/Game/GameMode/FL_Game.GetAIController` self) (`self.TargetLocation`))
  (return (`self.TargetLocation`)))

(fn `FN_ResetValues`
  (`|ExecutionSequence`
    (:`then_0`
      (set `self.Health` 100)
      (set `self.MaxHealth` 100))
    (:`then_1`
      (set `self.Shield` 100)
      (set `self.MaxShield` 100))
    (:`then_2`
      (set `self.Energy` 100)
      (set `self.MaxEnergy` 100))
    (:`then_3`
      (set `self.LightAttackDamage` 20)
      (set `self.LightAttackDamageCost` 30))
    (:`then_4`
      (set `self.StrongAttackDamage` 40)
      (set `self.StrongAttackDamageCost` 60))
    (:`then_5`
      (set `self.ShieldRegeneration` 30)
      (set `self.ShieldRegenerationCost` 40))
    (:`then_6`
      (set `self.EnergyRegeneration` 30))))

(fn `FN_SetTargetLocation`
  (params (TargetLocation :type "Vector Structure"))
  (set `self.TargetLocation` TargetLocation))

(fn `UserConstructionScript`
  (set `self.ShipStats` (`self.Widget`)))