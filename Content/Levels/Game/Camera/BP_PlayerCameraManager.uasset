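; BP_PlayerCameraManager is a player camera manager that keeps the screen black at level start and fades it in on request.
; StartFadeInEvent reasserts the black fade, slows the fade timeline's play rate and schedules FadeInEvent on a short delay timer.
; That timeline drives the manual camera fade amount each update, then calls the OnFadeInComplete event dispatcher when finished.
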(event `self.ReceiveBeginPlay`
  (`self.SetManualCameraFade` 1.0))

(event `StartFadeInEvent`
  (`|ExecutionSequence`
    (:`then_0`
      (`self.SetManualCameraFade` 1.0))
    (:`then_1`
      (`TimelineComponent.SetPlayRate` (`self.TL_FadeCamera`) (/ 1.0 3.0)))
    (:`then_2`
      (`KismetSystemLibrary.K2_SetTimerDelegate` (delegate `FadeInEvent`) 2.0))))

(event `FadeInEvent`
  (bind (_direction _fadeoutamount _fadeinamount) (`Timeline|TL_FadeCamera`)
    (:`Update`
      (`self.SetManualCameraFade` _fadeinamount))
    (:`Finished`
      (`self.OnFadeInCompleteEventDispatcher`))))

(fn `UserConstructionScript`)