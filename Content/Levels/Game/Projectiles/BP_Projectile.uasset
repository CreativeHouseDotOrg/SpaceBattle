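; BP_Projectile is a projectile fired by a ship that damages other ships on contact.
; Cylinder overlaps ignore the spawning ship, destroy the projectile on obstacles, and apply damage to other ships before destroying it.
; Each tick, it also destroys itself once its horizontal distance from the spawner's current position exceeds a maximum.
; Every destruction path first notifies the game through OnProjectileDestroyedEvent.
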(event `self.ReceiveTick`
  (params (DeltaSeconds :type "Float (single-precision)"))
  (if (> (`KismetMathLibrary.VSizeXY` (- (`SceneComponent.K2_GetComponentLocation` (`self.Cylinder`)) (`self.K2_GetActorLocation` (`self.SpawnerShip`)))) (`self.MaxDistanceFromSpawner`))
    (`/Game/Levels/Game/BP_Game.OnProjectileDestroyedEvent` (`/Game/Levels/Game/GameMode/FL_Game.GetGame`) :!label _label)
    (`self.K2_DestroyActor`)))

(event `self.Cylinder.OnComponentBeginOverlap`
  (params (OverlappedComponent :type "PrimitiveComponent Object Reference") (OtherActor :type "Actor Object Reference") (OtherComp :type "PrimitiveComponent Object Reference") (OtherBodyIndex :type Integer) (bFromSweep :type Boolean) (SweepResult :type "HitResult Structure (by ref)"))
  (if (not (== OtherActor (`self.SpawnerShip`)))
    (cast `/Game/Levels/Game/Prototyping/BP_Obstacle` OtherActor
      (:`then`
        (goto _label))
      (:`CastFailed`
        (bind _asbp_ship (cast `/Game/Levels/Game/Characters/Ship/BP_Ship` OtherActor))
        (`/Game/Levels/Game/Characters/Ship/BP_Ship.TakeDamageEvent` _asbp_ship (`self.Damage`))
        (goto _label)))))

(fn `UserConstructionScript`)