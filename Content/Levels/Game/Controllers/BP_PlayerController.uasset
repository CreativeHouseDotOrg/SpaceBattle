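; Player controller for a ship game that handles mouse camera movement and click-to-move of the current player ship.
; After the camera fade-in it enables mouse input and shows the HUD.
; Toggling the movement circle adds or removes the ship movement mapping context; clicks inside the ship's radius set a target with cursor FX, and a short press starts the move.
; Debug keys switch and focus the current player ship.
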(event `EnhancedInput|/Game/Levels/Game/Input/IA_SetDestination_Click`
  (params (ActionValue :type Boolean) (ElapsedSeconds :type "Float (double-precision)") (TriggeredSeconds :type "Float (double-precision)") (InputAction :type "InputAction Object Reference" :default "/Game/Levels/Game/Input/IA_SetDestination_Click.IA_SetDestination_Click"))
  (:`Triggered`
    (if (`self.GetIsMouseInShipRadius`)
      (`self.FN_MoveToTriggered`)))
  (:`Canceled`
    (if (`self.GetIsMouseInShipRadius`) :!label _label
      (`self.FN_MoveToCanceledCompleted` ElapsedSeconds)
      (`/Game/Levels/Game/UI/BP_HUD.ToggleRegenerateEnergyButtonEvent` (`/Game/Levels/Game/GameMode/FL_Game.GetHUD` 0) false)))
  (:`Completed`
    (goto _label)))

(event `EnhancedInput|/Game/Levels/Game/Input/IA_MoveCamera`
  (params (ActionValue :type Boolean) (ElapsedSeconds :type "Float (double-precision)") (TriggeredSeconds :type "Float (double-precision)") (InputAction :type "InputAction Object Reference" :default "/Game/Levels/Game/Input/IA_MoveCamera.IA_MoveCamera"))
  (bind (_locationx _locationy) (`self.GetMousePosition`))
  (bind _spectatorpawn (`/Game/Levels/Game/GameMode/FL_Game.GetSpectatorPawn` 0))
  (bind _returnvalue (`KismetMathLibrary.MakeVector2D` _locationx _locationy))
  (:`Started`
    (`/Game/Levels/Game/SpectatorPawn/BP_SpectatorPawn.StartMoveCameraEvent` _spectatorpawn _returnvalue))
  (:`Ongoing`
    (`/Game/Levels/Game/SpectatorPawn/BP_SpectatorPawn.MoveCameraEvent` _spectatorpawn _returnvalue))
  (:`Completed`
    (`/Game/Levels/Game/SpectatorPawn/BP_SpectatorPawn.ResetMovementVariablesEvent` _spectatorpawn)))

(event `EnableInputEvent`
  (`|ExecutionSequence`
    (:`then_0`
      (`/Game/Libraries/FL_MouseLib.FN_ActivateMouse`))
    (:`then_1`
      (`self.FN_AddInputContextMapping` "/Game/Levels/Game/Input/IMC_Player.IMC_Player"))))

(event `ToggleMovementCircleEvent`
  (params (bEnabled :type Boolean))
  (`self.FN_ToggleMovementCircle` bEnabled))

(event `Key|One`
  (params (Key :type "Key Structure"))
  (:`Released`
    (`/Game/Levels/Game/GameMode/BP_GameState.SetCurrentPlayerIndexEvent` (`/Game/Levels/Game/GameMode/FL_Game.GetGameState`) 0)
    (`/Game/Levels/Game/SpectatorPawn/BP_SpectatorPawn.FocusCurrentPlayerShipEvent` (`/Game/Levels/Game/GameMode/FL_Game.GetSpectatorPawn` 0) :!label _label_2)))

(event `Key|Two`
  (params (Key :type "Key Structure"))
  (:`Released`
    (`/Game/Levels/Game/GameMode/BP_GameState.SetCurrentPlayerIndexEvent` (`/Game/Levels/Game/GameMode/FL_Game.GetGameState`) 1)
    (goto _label_2)))

(event `InputVectorAxis|Mouse2D`
  (params (AxisValue :type "Vector Structure")))

(event `self.ReceiveBeginPlay`
  ;[0 0 0] Binds to the OnFadeInCompleteEventDispatcher which calls the "EnableInputEvent" aswell as the "ShowUIEvent" to enable the Controls after the FadeIn blending is finished.
  (add `/Game/Levels/Game/Camera/BP_PlayerCameraManager.OnFadeInCompleteEventDispatcher` (`/Game/Levels/Game/GameMode/FL_Game.GetPlayerCameraManager` 0) (delegate `ShowUIAndAllowInputsEvent`)))

(event `ShowUIAndAllowInputsEvent`
  ;[0 0 0] Binds to the OnFadeInCompleteEventDispatcher which calls the "EnableInputEvent" aswell as the "ShowUIEvent" to enable the Controls after the FadeIn blending is finished.
  (`|ExecutionSequence`
    (:`then_0`
      (`self.EnableInputEvent`))
    (:`then_1`
      (`/Game/Levels/Game/UI/BP_HUD.ShowUIEvent` (`/Game/Levels/Game/GameMode/FL_Game.GetHUD` 0)))))

(fn `FN_AddInputContextMapping`
  (params (MappingContext :type "InputMappingContext Object Reference"))
  (bind _returnvalue (subsystem `EnhancedInputLocalPlayerSubsystem`))
  (`/Engine/EditorBlueprintResources/StandardMacros.IsValid` _returnvalue
    (:`Is Valid`
      (`EnhancedInputSubsystemInterface.AddMappingContext` _returnvalue MappingContext 0 (struct)))))

(fn `FN_MoveToCanceledCompleted`
  (params (ElapsedSeconds :type "Float (double-precision)"))
  (if (< ElapsedSeconds (`self.PressedThreshold`))
    (`/Game/Levels/Game/Characters/Ship/BP_Ship.MoveToTargetLocationEvent` (`/Game/Levels/Game/GameMode/FL_Game.GetCurrentPlayerShip`))))

(fn `FN_MoveToTriggered`
  (bind (_hit _location) (`/Game/Libraries/FL_MouseLib.FN_GetLocationUnderCursor`))
  (if _hit
    (`/Game/Levels/Game/Characters/Ship/BP_Ship.FN_SetTargetLocation` (`/Game/Levels/Game/GameMode/FL_Game.GetCurrentPlayerShip`) _location)
    (`NiagaraFunctionLibrary.SpawnSystemAtLocation` (`self.FXCursor`) _location)))

(fn `FN_RemoveInputContextMapping`
  (params (MappingContext :type "InputMappingContext Object Reference"))
  (bind _returnvalue (subsystem `EnhancedInputLocalPlayerSubsystem`))
  (`/Engine/EditorBlueprintResources/StandardMacros.IsValid` _returnvalue
    (:`Is Valid`
      (`EnhancedInputSubsystemInterface.RemoveMappingContext` _returnvalue MappingContext (struct)))))

(fn `FN_ToggleMovementCircle`
  (params (bEnabled :type Boolean))
  (if bEnabled
    (`self.FN_AddInputContextMapping` "/Game/Levels/Game/Input/IMC_ShipMovement.IMC_ShipMovement")
    (`/Game/Levels/Game/Characters/Ship/BP_Ship.ShowMovementCircleEvent` (`/Game/Levels/Game/GameMode/FL_Game.GetCurrentPlayerShip`))
    (else
      (`self.FN_RemoveInputContextMapping` "/Game/Levels/Game/Input/IMC_ShipMovement.IMC_ShipMovement")
      (`/Game/Levels/Game/Characters/Ship/BP_Ship.HideMovementCircleEvent` (`/Game/Levels/Game/GameMode/FL_Game.GetCurrentPlayerShip`)))))

(fn `GetIsMouseInShipRadius`
  (returns (MouseIsInRadius :type Boolean) (Distance :type "Float (double-precision)"))
  (bind _ship (`/Game/Levels/Game/GameMode/FL_Game.GetCurrentPlayerShip`))
  (bind _returnvalue (`KismetMathLibrary.VSizeXY` (- (`.Location` (`/Game/Libraries/FL_MouseLib.FN_GetLocationUnderCursor`)) (`self.K2_GetActorLocation` _ship))))
  (return (<= _returnvalue (`/Game/Levels/Game/Characters/Ship/BP_Ship.GetMovementRadius` _ship)) _returnvalue))

(fn `UserConstructionScript`)