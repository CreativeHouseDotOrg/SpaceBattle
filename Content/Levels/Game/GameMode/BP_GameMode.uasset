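; BP_GameMode is a game mode that gathers players and starts the match on all clients once the required count has joined.
; PostLogin stores each player controller and registers its player state with the GameState, while BeginPlay creates additional local players up to GameRules.PlayersNeeded.
; ReadyToStartMatch compares the controller count to that number.
; The InProgress match state fires a dispatcher, bound to call StartGameEvent on the GameState with GameRules.
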(event `self.K2_PostLogin`
  (params (NewPlayer :type "PlayerController Object Reference"))
  ;[0 0 0] When a new Player Connects then
  ; Add the "BP_PlayerController" to the PlayerControllers Collection and
  ; Add the "BP_PlayerState" to the PlayerStates Collection which is inside of BP_GameState
  (bind _asbp_player_controller (cast `/Game/Levels/Game/Controllers/BP_PlayerController` NewPlayer))
  (`KismetArrayLibrary.Array_Add` (`self.PlayerControllers`) _asbp_player_controller)
  (`/Game/Levels/Game/GameMode/BP_GameState.FN_AddPlayerState` (`/Game/Levels/Game/GameMode/FL_Game.GetGameState`) (`Controller.PlayerState` _asbp_player_controller)))

(event `self.K2_OnSetMatchState`
  (params (NewState :type Name))
  ;[0 0 0] Check the new State of the Game
  ;
  ; The "NewState"-Name Property will change its value to "InProgress" if the "ReadyToStartMatch"-Function returns true
  (if (== NewState "InProgress")
    (`self.ED_OnMatchReady`)))

(event `self.ReceiveBeginPlay`
  (`|ExecutionSequence`
    (:`then_0`
      ;[0 0 0] When the MatchReady EventDispatcher is being called,
      ; then the StartAllClients Event will call "StartGameEvent" on the GameState
      ; This basically tells all Clients to Start the Game
      (add `self.ED_OnMatchReady` (delegate `StartAllClientsEvent`)))
    (:`then_1`
      ;[0 0 0] Spawn the local players
      (for _index (range 1 (`.PlayersNeeded_8_E8998C374CF7D5C80E1A179F1576CDFC` (break `/Game/Levels/Game/GameMode/GameRulesStruct` (`self.GameRules`))))
        (`GameplayStatics.CreatePlayer` _index)))))

(event `StartAllClientsEvent`
  ;[0 0 0] When the MatchReady EventDispatcher is being called,
  ; then the StartAllClients Event will call "StartGameEvent" on the GameState
  ; This basically tells all Clients to Start the Game
  (`/Game/Levels/Game/GameMode/BP_GameState.StartGameEvent` (`/Game/Levels/Game/GameMode/FL_Game.GetGameState`) (`self.GameRules`)))

(fn `ReadyToStartMatch`
  (returns (ReturnValue :type Boolean))
  (bind _output_get (set `self.GameIsReady` (== (`KismetArrayLibrary.Array_Length` (`self.PlayerControllers`)) (`.PlayersNeeded_8_E8998C374CF7D5C80E1A179F1576CDFC` (break `/Game/Levels/Game/GameMode/GameRulesStruct` (`self.GameRules`))))))
  (return _output_get))

(fn `UserConstructionScript`)