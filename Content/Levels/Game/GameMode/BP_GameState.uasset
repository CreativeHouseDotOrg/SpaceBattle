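; BP_GameState is the game state for a turn-based game with player ships, tracking rules, round, current player index and player states.
; Starting a game sets the rules and round one, notifies every player state, resets all ships, then starts the game object.
; Ending a turn advances the player index, wrapping to the first player and incrementing the round after the last.
; Setters broadcast event dispatchers when rules, round or player change.
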(event `StartGameEvent`
  (params (GameRules :type "/Game/Levels/Game/GameMode/GameRulesStruct Structure"))
  (`self.FN_StartGame` GameRules))

(event `EndTurnEvent`
  (`self.FN_EndTurn`))

(fn `FN_AddPlayerState`
  (params (NewPlayerState :type "PlayerState Object Reference"))
  (bind _asbp_player_state (cast `/Game/Levels/Game/Player/BP_PlayerState` NewPlayerState))
  (`KismetArrayLibrary.Array_Add` (`self.PlayerStates`) _asbp_player_state)
  (return))

(fn `FN_EndTurn`
  (if (== (`self.CurrentPlayerIndex`) (- (`KismetArrayLibrary.Array_Length` (`self.PlayerStates`)) 1))
    (`self.FN_SetCurrentRound` (+ (`self.CurrentRound`) 1))
    (`self.FN_SetCurrentPlayerIndex` 0)
    (else
      (`self.FN_SetCurrentPlayerIndex` (+ (`self.CurrentPlayerIndex`) 1)))))

(fn `FN_SetCurrentGameRules`
  (params (Rules :type "/Game/Levels/Game/GameMode/GameRulesStruct Structure"))
  (bind _output_get (set `self.CurrentGameRules` Rules))
  (`self.ED_OnCurrentGameRulesChanged` _output_get))

(fn `FN_SetCurrentPlayerIndex`
  (params (NewPlayerIndex :type Integer))
  (bind _output_get (set `self.CurrentPlayerIndex` NewPlayerIndex))
  (`self.ED_OnPlayerIndexChanged` _output_get))

(fn `FN_SetCurrentRound`
  (params (CurrentRound :type Integer))
  (bind _output_get (set `self.CurrentRound` CurrentRound))
  (`self.ED_OnCurrentRoundChanged` _output_get))

(fn `FN_StartGame`
  (params (Rules :type "/Game/Levels/Game/GameMode/GameRulesStruct Structure"))
  (`self.FN_SetCurrentGameRules` Rules)
  (`|ExecutionSequence`
    (:`then_0`
      (`self.FN_SetCurrentRound` 1))
    (:`then_1`
      (bind _playerstate (`/Game/Levels/Game/GameMode/ML_Game.ForEachPlayerStates`)
        (:`Loop Body`
          (`/Game/Levels/Game/Player/BP_PlayerState.StartGameEvent` _playerstate))))
    (:`then_2`
      (bind _playership (`/Game/Levels/Game/GameMode/ML_Game.ForEachPlayerShips`)
        (:`LoopBody`
          (`/Game/Levels/Game/Characters/Ship/BP_Ship.ResetValuesEvent` _playership))))
    (:`then_3`
      (`/Game/Levels/Game/BP_Game.StartGame` (`/Game/Levels/Game/GameMode/FL_Game.GetGame`)))))

(fn `GetGameRules`
  (returns (CurrentGameRules :type "/Game/Levels/Game/GameMode/GameRulesStruct Structure"))
  (return (`self.CurrentGameRules`)))

(fn `UserConstructionScript`)