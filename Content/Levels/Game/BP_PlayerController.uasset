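; Player controller for the game level that starts up the camera and mouse controls.
; BeginPlay enables mouse events and asks BP_PlayerCameraManager to set up the first camera.
; ClientInitialize, in sequence, fills the screen with a solid color, shows the cursor, resets the active camera to its default transform and fades in.
; Camera work is delegated to the camera manager through small wrapper functions, and a missing active camera prints an error.
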(event `self.ReceiveBeginPlay`
  (`/Game/Libraries/MouseControlsLib.EnableMouseEvent` (`self.MouseControlsLib`))
  (`self.FN_InitCamera`))

(event `ClientInitialize`
  (`|ExecutionSequence`
    (:`then_0`
      (bind _cameramanager (`self.FN_GetPlayerCameraManager`))
      (`/Game/Levels/Game/BP_PlayerCameraManager.FillScreenWithSolidColorEvent` _cameramanager))
    (:`then_1`
      (`self.FN_ActivateMouse`))
    (:`then_2`
      (`self.FN_CameraSetDefaultTransform`))
    (:`then_3`
      (`self.FN_FadeCamera` true))))

(fn `FN_ActivateMouse`
  (set `PlayerController.bShowMouseCursor` true (`GameplayStatics.GetPlayerController` 0))
  (return))

(fn `FN_CameraSetDefaultTransform`
  (bind _cameramanager (`self.FN_GetPlayerCameraManager`))
  (bind _activecamera (`/Game/Levels/Game/BP_PlayerCameraManager.FN_GetActiveCamera` _cameramanager))
  (`/Engine/EditorBlueprintResources/StandardMacros.IsValid` _activecamera
    (:`Is Valid`
      (`/Game/Levels/Game/BP_GameCamera.SetDefaultCameraTransformEvent` _activecamera)
      (return))
    (:`Is Not Valid`
      (`/Game/Libraries/PrintLib.PrintError` (`self.PrintLib`) "No Active Camera set!" 20.0))))

(fn `FN_FadeCamera`
  (params (bFadeIn :type Boolean))
  (bind _cameramanager (`self.FN_GetPlayerCameraManager`))
  (`/Game/Levels/Game/BP_PlayerCameraManager.FadeInOutEvent` _cameramanager 2.0 bFadeIn)
  (return))

(fn `FN_GetPlayerCameraManager`
  (returns (CameraManager :type "/Game/Levels/Game/BP_PlayerCameraManager Object Reference"))
  (bind _asbp_player_camera_manager (cast `/Game/Levels/Game/BP_PlayerCameraManager` (`GameplayStatics.GetPlayerCameraManager` 0)))
  (return _asbp_player_camera_manager))

(fn `FN_InitCamera`
  (bind _cameramanager (`self.FN_GetPlayerCameraManager`))
  (`/Game/Levels/Game/BP_PlayerCameraManager.InitFirstCameraEvent` _cameramanager))

(fn `UserConstructionScript`)