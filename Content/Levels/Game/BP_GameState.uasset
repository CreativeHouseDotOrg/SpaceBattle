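; BP_GameState is a game state Blueprint that tracks the registered players and the current player index.
; Player states are cast to BP_PlayerState before being added to an array, and starting the game calls the start-game event on each one.
; Setting the current player index fires an event dispatcher with the new value, so listeners can react to player changes.
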(fn `FN_AddPlayerState`
  (params (NewPlayerState :type "PlayerState Object Reference"))
  (bind _asbp_player_state (cast `/Game/Levels/Game/BP_PlayerState` NewPlayerState))
  (`KismetArrayLibrary.Array_Add` (`self.PlayerStates`) _asbp_player_state)
  (return))

(fn `FN_SetCurrentPlayerIndex`
  (params (NewPlayerIndex :type Integer))
  (bind _output_get (set `self.CurrentPlayerIndex` NewPlayerIndex))
  (`self.ED_OnPlayerIndexChanged` _output_get))

(fn `FN_StartGame`
  (for _array_element (`self.PlayerStates`)
    (`/Game/Levels/Game/BP_PlayerState.StartGameEvent` _array_element)))

(fn `UserConstructionScript`)