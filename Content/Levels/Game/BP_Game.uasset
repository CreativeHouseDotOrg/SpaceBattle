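; Match controller for a turn-based ship battle, running setup, turns and game over.
; StartGame spawns the arena, random obstacles, start positions (rerolled on obstacle overlap) and one ship per start.
; Bind subgraphs route GameState, ship and HUD dispatchers into handlers for actions and turn changes, rebinding stat updates to the active ship.
; Each turn shows a notification, spawns pickups and runs a countdown that pauses during movement and projectile flight.
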(event `OnShipMovementStartedEvent`
  ;[0 0 0] This event gets called when the Ship has started moving towards the target location.
  (`self.FN_OnShipMovementStarted`))

(event `OnPlayerIndexChangedEvent`
  (params (PreviousPlayerShip :type "/Game/Levels/Game/Characters/Ship/BP_Ship Object Reference"))
  ;[0 0 0] Gets called when the Player Index has been changed. (When the player has ended the turn and when it's the next players turn!
  (`self.FN_DeactivateShip` PreviousPlayerShip)
  (`self.ShowTurnNotificationEvent`)
  (`self.FN_ActivateCurrentShip`))

(event `OnActionBarInteractionEvent`
  (params (Interaction :type "/Game/Levels/Game/Enums/EShipInteraction Enum" :default "NewEnumerator0"))
  ;[0 0 0] Switching through the EShipInteraction Enum when a Action Button in the UI is pressed that contains a EShipInteraction.
  (switch `/Game/Levels/Game/Enums/EShipInteraction` Interaction
    (:`NewEnumerator0`
      (`self.ToggleShipMovementEvent`))
    (:`NewEnumerator1`
      (`self.ToggleAttackEvent` "NewEnumerator0"))
    (:`NewEnumerator2`
      (`self.ToggleAttackEvent` "NewEnumerator1"))
    (:`NewEnumerator3`
      (`self.RegenerateShieldEvent`))
    (:`NewEnumerator4`
      (`self.RegenerateEnergyEvent`))))

(event `StartGame`
  (`|ExecutionSequence`
    (:`then_1`
      (`|ExecutionSequence`
        (:`then_0`
          (add `self.ED_OnPlayerShipsSpawned` (delegate `OnPlayerShipsSpawnedBindEvent`)))
        (:`then_1`
          (add `/Game/Levels/Game/GameMode/BP_GameState.ED_OnPlayerIndexChanged` (`/Game/Levels/Game/GameMode/FL_Game.GetGameState`) (delegate `OnPlayerIndexChangedBindEvent`)))
        (:`then_2`
          (add `/Game/Levels/Game/UI/BP_HUD.ED_OnInteraction` (`/Game/Levels/Game/GameMode/FL_Game.GetCurrentHUD`) (delegate `OnActionBarInteractionBindEvent`)))
        (:`then_3`
          (add `/Game/Levels/Game/GameMode/BP_GameState.ED_OnCurrentRoundChanged` (`/Game/Levels/Game/GameMode/FL_Game.GetGameState`) (delegate `OnCurrentRoundChangedBindEvent`)))))
    (:`then_2`
      (`self.FN_SpawnArena` 200 200)
      (`self.HandlePlayerStartPositionsEvent`))))

(event `OnPlayerShipsSpawnedBindEvent`
  (`|ExecutionSequence`
    (:`then_0`
      (`self.OnPlayerShipsSpawnedEvent`))
    (:`then_1`
      (bind _playership (`/Game/Levels/Game/GameMode/ML_Game.ForEachPlayerShips`)
        (:`LoopBody`
          (add `/Game/Levels/Game/Characters/Ship/BP_Ship.ED_OnMovementStarted` _playership (delegate `OnMovementStartedBindEvent`)))))
    (:`then_2`
      (bind _playership_2 (`/Game/Levels/Game/GameMode/ML_Game.ForEachPlayerShips`)
        (:`LoopBody`
          (add `/Game/Levels/Game/Characters/Ship/BP_Ship.ED_OnMovementCompleted` _playership_2 (delegate `OnMovementCompletedBindEvent`)))))))

(event `OnActionBarInteractionBindEvent`
  (params (Interaction :type "/Game/Levels/Game/Enums/EShipInteraction Enum" :default "NewEnumerator0"))
  (`self.OnActionBarInteractionEvent` Interaction))

(event `OnPlayerIndexChangedBindEvent`
  (params (NewPlayerIndex :type Integer) (OldPlayerIndex :type Integer))
  (bind _ship (`/Game/Levels/Game/GameMode/FL_Game.GetPlayerShip` OldPlayerIndex))
  (remove `/Game/Levels/Game/Characters/Ship/BP_Ship.ED_OnShipStatsChanged` _ship (delegate `OnShipStatsChangedBindEvent`))
  (add `/Game/Levels/Game/Characters/Ship/BP_Ship.ED_OnShipStatsChanged` (`/Game/Levels/Game/GameMode/FL_Game.GetPlayerShip` NewPlayerIndex) (delegate `OnShipStatsChangedBindEvent`))
  (`self.OnPlayerIndexChangedEvent` _ship))

(event `OnShipStatsChangedBindEvent`
  (params (Ship :type "/Game/Levels/Game/Characters/Ship/BP_Ship Object Reference") (ShipStats :type "/Game/Levels/Game/Structs/ShipStatsStruct Structure"))
  (`self.OnShipStatsChangedEvent` Ship ShipStats))

(event `OnMovementCompletedBindEvent`
  (`self.OnShipMovementCompletedEvent`))

(event `OnMovementStartedBindEvent`
  (`self.OnShipMovementStartedEvent`))

(event `OnCurrentRoundChangedBindEvent`
  (params (CurrentRound :type Integer))
  (`self.OnCurrentRoundChangedEvent` CurrentRound))

(event `OnShipStatsChangedEvent`
  (params (AffectedShip :type "/Game/Levels/Game/Characters/Ship/BP_Ship Object Reference") (NewShipStats :type "/Game/Levels/Game/Structs/ShipStatsStruct Structure"))
  ;[0 0 0] Gets called when one of the player's ship's stats have been modified.
  (`/Game/Levels/Game/UI/BP_HUD.SetActiveShipInUI` (`/Game/Levels/Game/GameMode/FL_Game.GetHUD` 0) AffectedShip))

(event `OnShipMovementCompletedEvent`
  ;[0 0 0] This event will get called then the Ship has either reached its target location or the path was blocked while flying towards the target location.
  (`self.FN_OnShipMovementCompleted`))

(event `ToggleShipStatsWidgetsEvent`
  (params (bEnabled :type Boolean))
  ;[0 0 0] Toggles the ShipStats Widget above all Ships
  (for _array_element (`self.ShipArray`)
    (`/Game/Levels/Game/Characters/Ship/BP_Ship.ToggleShipStats` _array_element bEnabled)))

(event `OnProjectileFiredEvent`
  ;[0 0 0] This event will get called when the projectile has been fired from the ship.
  (`self.FN_OnProjectileFired`))

(event `ToggleShipMovementEvent`
  (bind _playercontroller (`/Game/Levels/Game/GameMode/FL_Game.GetPlayerController` 0))
  ;[0 0 0] Toggles the Ship Movement Circle
  (set `/Game/Levels/Game/Controllers/BP_PlayerController.EAttackStrength` "NewEnumerator2" _playercontroller)
  (`/Game/Levels/Game/Controllers/BP_PlayerController.ToggleShipAttackEvent` _playercontroller "NewEnumerator2")
  (`/Game/Levels/Game/Controllers/BP_PlayerController.ToggleShipMovementEvent` _playercontroller (not (`/Game/Levels/Game/Controllers/BP_PlayerController.bShowMovementRadius` _playercontroller))))

(event `OnShipDestroyedEvent`
  (params (DestroyedShip :type "/Game/Levels/Game/Characters/Ship/BP_Ship Object Reference"))
  ;[0 0 0] Fires when a Ship gets destroyed.
  ;
  ; WTF Explanation:
  ; Removes the Object Reference of the destroyed Ship from the ShipArray and then fixes the issue with the shifting CurrentPlayerIndex
  (`self.FN_DestroyShip` DestroyedShip)
  (`self.FN_CheckIfMatchIsOver`))

(event `OnProjectileDestroyedEvent`
  ;[0 0 0] This event will get called when the projectile has been destroyed.
  (`self.FN_OnProjectileDestroyed`))

(event `HandlePlayerStartPositionsEvent`
  ;[0 0 0] Handle the spawning of the PlayerStartPositions
  (`self.FN_CleanUpSpawnStartPoints`)
  (`self.FN_SpawnStartPositions` (`/Game/Levels/Game/GameMode/FL_Game.GetNumPlayers`))
  (bind _bisoverlapping (`self.FN_CheckIfStartPositionsOverlap`))
  (if _bisoverlapping
    (`self.HandlePlayerStartPositionsEvent`)
    (else
      (`self.SpawnPlayerShipsEvent`))))

(event `ToggleAttackEvent`
  (params (EAttackStrength :type "/Game/Levels/Game/Enums/EAttackStrength Enum" :default "NewEnumerator2"))
  (bind _playercontroller (`/Game/Levels/Game/GameMode/FL_Game.GetPlayerController` 0))
  (bind _playercontroller_2 (`/Game/Levels/Game/GameMode/FL_Game.GetPlayerController` 0))
  ;[0 0 0] Toggles the Attack Circle
  (`/Game/Levels/Game/Controllers/BP_PlayerController.ToggleShipMovementEvent` _playercontroller false)
  (if (`|EnumInequality` EAttackStrength (`/Game/Levels/Game/Controllers/BP_PlayerController.EAttackStrength` _playercontroller))
    (set `/Game/Levels/Game/Controllers/BP_PlayerController.EAttackStrength` EAttackStrength _playercontroller_2)
    (`/Game/Levels/Game/Controllers/BP_PlayerController.ToggleShipAttackEvent` (`/Game/Levels/Game/GameMode/FL_Game.GetPlayerController` 0) (`/Game/Levels/Game/Controllers/BP_PlayerController.EAttackStrength` _playercontroller_2))
    (else
      (bind _output_get (set `/Game/Levels/Game/Controllers/BP_PlayerController.EAttackStrength` "NewEnumerator2" _playercontroller))
      (`/Game/Levels/Game/Controllers/BP_PlayerController.ToggleShipAttackEvent` _playercontroller _output_get))))

(event `EndTurnEvent`
  ;[0 0 0] Gets fired when the player ends his turn.
  (`self.FN_EndTurn`)
  (`/Game/Levels/Game/Spawners/Pickups/BP_PickupSpawner.CleanUpPickupsEvent` (`self.BP_PickupSpawner`)))

(event `SpawnPlayerShipsEvent`
  ;[0 0 0] Spawn the PlayerShips
  (`self.FN_SpawnShips`)
  (`self.ED_OnPlayerShipsSpawned`))

(event `GameOverEvent`
  ;[0 0 0] Gets called when the Game is Over
  (`self.FN_GameOver`))

(event `RegenerateShieldEvent`
  ;[0 0 0] Performs the Shield Regeneration
  (`/Game/Levels/Game/Controllers/BP_PlayerController.UntoggleAllActionsEvent` (`/Game/Levels/Game/GameMode/FL_Game.GetPlayerController` 0))
  (`/Game/Levels/Game/Characters/Ship/BP_Ship.RegenerateShieldEvent` (`/Game/Levels/Game/GameMode/FL_Game.GetCurrentPlayerShip`))
  (`/Game/Levels/Game/UI/BP_HUD.ToggleRegenerateEnergyButtonEvent` (`/Game/Levels/Game/GameMode/FL_Game.GetHUD` 0) false))

(event `ShowTurnNotificationEvent`
  ;[0 0 0] Shows the TurnNotification Widget for a couple of seconds and then deactivates it automatically. After it is deactivated it will also resume the gameplay.
  (`/Game/Levels/Game/UI/BP_HUD.ShowTurnNotificationEvent` (`/Game/Levels/Game/GameMode/FL_Game.GetHUD` 0) (`/Game/Levels/Game/Characters/Ship/BP_Ship.ShipId` (`/Game/Levels/Game/GameMode/FL_Game.GetCurrentPlayerShip`)))
  (`KismetSystemLibrary.K2_SetTimerDelegate` (delegate `HideTurnNotificationEvent`) 3.0)
  (`self.FN_DeactivateGameplay`))

(event `HideTurnNotificationEvent`
  ;[0 0 0] Shows the TurnNotification Widget for a couple of seconds and then deactivates it automatically. After it is deactivated it will also resume the gameplay.
  (`self.FN_ActivateGameplay`)
  (`/Game/Levels/Game/Spawners/Pickups/BP_PickupSpawner.SpawnPickupsEvent` (`self.BP_PickupSpawner`) 6 10))

(event `RegenerateEnergyEvent`
  ;[0 0 0] Performs the Energy Regeneration
  (`/Game/Levels/Game/Characters/Ship/BP_Ship.RegenerateEnergyEvent` (`/Game/Levels/Game/GameMode/FL_Game.GetCurrentPlayerShip`))
  (`self.EndTurnEvent`))

(event `OnPlayerShipsSpawnedEvent`
  ;[0 0 0] This event will get called after the PlayerShips are spawned.
  (`|ExecutionSequence`
    (:`then_0`
      (bind _playership (`/Game/Levels/Game/GameMode/ML_Game.ForEachPlayerShips`)
        (:`LoopBody`
          (`/Game/Levels/Game/Characters/Ship/BP_Ship.ResetValuesEvent` _playership))))
    (:`then_1`
      (`self.ToggleShipStatsWidgetsEvent` true))
    (:`then_2`
      (`/Game/Levels/Game/UI/BP_HUD.ToggleAllButtonsEnabledEvent` (`/Game/Levels/Game/GameMode/FL_Game.GetHUD` 0) false))
    (:`then_3`
      ;;[0 0 0] Starts the FadeIn blend
      (`/Game/Levels/Game/UI/BP_HUD.StartFadeInEvent` (`/Game/Levels/Game/GameMode/FL_Game.GetHUD` 0) 2.0 1.0))))

(event `ResetTimerEvent`
  ;[0 0 0] Resets the Time and starts the Timer that counts the Time down.
  (`self.FN_ResetTimer`))

(event `RunTimerEvent`
  ;[0 0 0] Runs the Timer
  (bind _returnvalue (`KismetSystemLibrary.K2_SetTimerDelegate` (delegate `TimerTickEvent`) 0.1 true))
  (set `self.Timer` _returnvalue))

(event `TimerTickEvent`
  (bind _gamestate (`/Game/Levels/Game/GameMode/FL_Game.GetGameState`))
  (bind _timeleft (`/Game/Levels/Game/GameMode/BP_GameState.TimeLeft` _gamestate))
  ;[0 0 0] Runs the Timer
  (`/Game/Levels/Game/GameMode/BP_GameState.SetSecondsLeftEvent` _gamestate (- _timeleft 0.1))
  (if (== _timeleft 0.0)
    (`self.EndTurnEvent`)))

(event `StopTimerEvent`
  ;[0 0 0] Stops (well... actually pauses) the Timer
  (`KismetSystemLibrary.K2_ClearAndInvalidateTimerHandle` (`self.Timer`)))

(event `OnCurrentRoundChangedEvent`
  (params (CurrentRound :type Integer)))

(event `InitMediaPlayer`
  (bind _returnvalue (`MediaSoundComponent.GetMediaPlayer` (`self.MSC_MusicPlayer`)))
  ;[0 0 0] Starts the Music
  (bind _returnvalue_2 (`AddComponent|NODE_AddMediaSoundComponent-0`))
  (bind _output_get (set `self.MSC_MusicPlayer` _returnvalue_2))
  (`MediaSoundComponent.SetMediaPlayer` _output_get "/Game/Music/MP_MusicPlayer.MP_MusicPlayer")
  (`MediaPlayer.OpenSource` _returnvalue "/Game/Music/Foregone_Destruction__Facing_Worlds__-_Unreal_Tournament.Foregone_Destruction__Facing_Worlds__-_Unreal_Tournament")
  (`MediaPlayer.Play` _returnvalue))

(event `OnFadeInCompletedEvent`
  ;[0 0 0] This Event gets called when the FadeIn was completed.
  (`|ExecutionSequence`
    (:`then_0`
      (`self.FN_CheckIfMatchIsOver`))
    (:`then_1`
      (`/Game/Levels/Game/GameMode/BP_GameState.SetCurrentPlayerIndexEvent` (`/Game/Levels/Game/GameMode/FL_Game.GetGameState`) 0))))

(fn `FN_ActivateCurrentShip`
  (`|ExecutionSequence`
    (:`then_0`
      (`/Game/Levels/Game/UI/BP_HUD.SetActiveShipInUI` (`/Game/Levels/Game/GameMode/FL_Game.GetHUD` 0) (`/Game/Levels/Game/GameMode/FL_Game.GetCurrentPlayerShip`)))
    (:`then_1`
      ;[0 0 0] Focuses the current Player Ship
      (`/Game/Levels/Game/SpectatorPawn/BP_SpectatorPawn.FocusCurrentPlayerShipEvent` (`/Game/Levels/Game/GameMode/FL_Game.GetSpectatorPawn` 0)))
    (:`then_2`
      (`/Game/Levels/Game/Characters/Ship/BP_Ship.RegenerateEnergyEvent` (`/Game/Levels/Game/GameMode/FL_Game.GetCurrentPlayerShip`)))))

(fn `FN_ActivateGameplay`
  (`|ExecutionSequence`
    (:`then_0`
      (`/Game/Levels/Game/UI/BP_HUD.HideTurnNotificationEvent` (`/Game/Levels/Game/GameMode/FL_Game.GetHUD` 0)))
    (:`then_1`
      (`/Game/Levels/Game/UI/BP_HUD.ToggleAllButtonsEnabledEvent` (`/Game/Levels/Game/GameMode/FL_Game.GetHUD` 0) true)
      (`/Game/Levels/Game/UI/BP_HUD.ShowGameHUDEvent` (`/Game/Levels/Game/GameMode/FL_Game.GetHUD` 0))
      (`/Game/Levels/Game/Controllers/BP_PlayerController.EnableInputEvent` (`/Game/Levels/Game/GameMode/FL_Game.GetPlayerController` 0))
      (`self.ResetTimerEvent`))))

(fn `FN_CheckIfMatchIsOver`
  (if (== (`KismetArrayLibrary.Array_Length` (`self.ShipArray`)) 1)
    (`/Game/Levels/Game/GameMode/BP_GameState.GameOverEvent` (`/Game/Levels/Game/GameMode/FL_Game.GetGameState`))))

(fn `FN_CheckIfStartPositionsOverlap`
  (returns (bIsOverlapping :type Boolean))
  (locals (bIsInvalid :type Boolean))
  (for _array_element (`self.PlayerStarts`)
    (if (`/Game/Levels/Game/Player/BP_PlayerStart.bIsOverlappingObstacle` _array_element)
      (set `local.bIsInvalid` true)))
  (`|ExecutionSequence`
    (:`then_0`
      (if (`local.bIsInvalid`)
        (`KismetSystemLibrary.PrintString` "Invalid spawn point detected. Preparing for Autofix" true true (struct :`R` 1.0 :`B` 0.069748 :`A` 1.0))))
    (:`then_1`
      (return (`local.bIsInvalid`)))))

(fn `FN_CleanUpSpawnStartPoints`
  (bind _playerstarts (`self.PlayerStarts`))
  (for _array_element _playerstarts
    (`self.K2_DestroyActor` _array_element))
  (`KismetArrayLibrary.Array_Clear` _playerstarts))

(fn `FN_DeactivateGameplay`
  (`/Game/Levels/Game/UI/BP_HUD.HideGameHUDEvent` (`/Game/Levels/Game/GameMode/FL_Game.GetHUD` 0))
  (`/Game/Levels/Game/Controllers/BP_PlayerController.DisableInputEvent` (`/Game/Levels/Game/GameMode/FL_Game.GetPlayerController` 0))
  (`self.StopTimerEvent`))

(fn `FN_DeactivateShip`
  (params (ShipToDeactivate :type "/Game/Levels/Game/Characters/Ship/BP_Ship Object Reference"))
  (`/Game/Levels/Game/Characters/Ship/BP_Ship.HideMovementCircleEvent` ShipToDeactivate)
  (`/Game/Levels/Game/Characters/Ship/BP_Ship.HideAttackCircleEvent` ShipToDeactivate))

(fn `FN_DestroyShip`
  (params (DestroyedShip :type "/Game/Levels/Game/Characters/Ship/BP_Ship Object Reference"))
  (`KismetArrayLibrary.Array_RemoveItem` (`self.ShipArray`) DestroyedShip)
  (`/Game/Levels/Game/GameMode/BP_GameState.FixCurrentPlayerIndexEvent` (`/Game/Levels/Game/GameMode/FL_Game.GetGameState`))
  (return))

(fn `FN_EndTurn`
  (`/Game/Levels/Game/Controllers/BP_PlayerController.UntoggleAllActionsEvent` (`/Game/Levels/Game/GameMode/FL_Game.GetPlayerController` 0))
  (`/Game/Levels/Game/UI/BP_HUD.ToggleAllButtonsEnabledEvent` (`/Game/Levels/Game/GameMode/FL_Game.GetHUD` 0) false)
  (`/Game/Levels/Game/GameMode/BP_GameState.EndTurnEvent` (`/Game/Levels/Game/GameMode/FL_Game.GetGameState`)))

(fn `FN_GameOver`
  (bind _playercontroller (`/Game/Levels/Game/GameMode/FL_Game.GetPlayerController` 0))
  (`/Game/Levels/Game/UI/BP_HUD.ToggleAllButtonsEnabledEvent` (`/Game/Levels/Game/GameMode/FL_Game.GetHUD` 0) false)
  (`/Game/Levels/Game/Controllers/BP_PlayerController.ToggleShipMovementEvent` _playercontroller false)
  (`/Game/Levels/Game/Controllers/BP_PlayerController.ToggleShipAttackEvent` _playercontroller "NewEnumerator2")
  (`/Game/Levels/Game/UI/BP_HUD.ShowGameOverScreenEvent` (`/Game/Levels/Game/GameMode/FL_Game.GetHUD` 0)))

(fn `FN_OnProjectileDestroyed`
  (bind _playercontroller (`/Game/Levels/Game/GameMode/FL_Game.GetPlayerController` 0))
  (`/Game/Levels/Game/Controllers/BP_PlayerController.ToggleShipAttackEvent` _playercontroller (`/Game/Levels/Game/Controllers/BP_PlayerController.EAttackStrength` _playercontroller))
  (`/Game/Levels/Game/UI/BP_HUD.ToggleAllButtonsEnabledEvent` (`/Game/Levels/Game/GameMode/FL_Game.GetHUD` 0) true)
  (`/Game/Levels/Game/UI/BP_HUD.ToggleRegenerateEnergyButtonEvent` (`/Game/Levels/Game/GameMode/FL_Game.GetHUD` 0) false)
  (`self.RunTimerEvent`))

(fn `FN_OnProjectileFired`
  (`self.StopTimerEvent`)
  (`/Game/Levels/Game/Controllers/BP_PlayerController.ToggleShipAttackEvent` (`/Game/Levels/Game/GameMode/FL_Game.GetPlayerController` 0) "NewEnumerator2")
  (`/Game/Levels/Game/UI/BP_HUD.ToggleAllButtonsEnabledEvent` (`/Game/Levels/Game/GameMode/FL_Game.GetHUD` 0) false))

(fn `FN_OnShipMovementCompleted`
  (`/Game/Levels/Game/Controllers/BP_PlayerController.ToggleShipMovementEvent` (`/Game/Levels/Game/GameMode/FL_Game.GetPlayerController` 0) (`/Game/Levels/Game/Characters/Ship/BP_Ship.GetCanPerformMovement` (`/Game/Levels/Game/GameMode/FL_Game.GetCurrentPlayerShip`)))
  (`/Game/Levels/Game/UI/BP_HUD.ToggleAllButtonsEnabledEvent` (`/Game/Levels/Game/GameMode/FL_Game.GetHUD` 0) true)
  (`/Game/Levels/Game/UI/BP_HUD.ToggleRegenerateEnergyButtonEvent` (`/Game/Levels/Game/GameMode/FL_Game.GetHUD` 0) false)
  (`self.RunTimerEvent`))

(fn `FN_OnShipMovementStarted`
  (`self.StopTimerEvent`)
  (`/Game/Levels/Game/Controllers/BP_PlayerController.ToggleShipMovementEvent` (`/Game/Levels/Game/GameMode/FL_Game.GetPlayerController` 0) false)
  (`/Game/Levels/Game/UI/BP_HUD.ToggleAllButtonsEnabledEvent` (`/Game/Levels/Game/GameMode/FL_Game.GetHUD` 0) false))

(fn `FN_ResetTimer`
  (bind _gamestate (`/Game/Levels/Game/GameMode/FL_Game.GetGameState`))
  (bind (_currentgamerules_rounds _currentgamerules_timeperround) (break `/Game/Levels/Game/Structs/GameRulesStruct` (`/Game/Levels/Game/GameMode/BP_GameState.CurrentGameRules` _gamestate)))
  (`/Game/Levels/Game/GameMode/BP_GameState.SetSecondsLeftEvent` _gamestate _currentgamerules_timeperround)
  (`self.RunTimerEvent`))

(fn `FN_SetNavMeshBounds`
  (params (Scale :type "Vector Structure"))
  (bind (_x _y) (`KismetMathLibrary.BreakVector3f` Scale))
  (`self.SetActorScale3D` (`self.NavMeshBoundsVolume`) (`KismetMathLibrary.MakeVector` _x _y 1.0))
  (return))

(fn `FN_SpawnArena`
  (params (SizeX :type Integer) (SizeY :type Integer))
  (bind _returnvalue (`|SpawnActorFromClass` "/Game/Levels/Game/Prototyping/BP_Floor.BP_Floor_C" (`KismetMathLibrary.MakeTransform` (0.0 0.0 0.0) (struct) (`KismetMathLibrary.MakeVector` (`KismetMathLibrary.Conv_IntToDouble` SizeX) (`KismetMathLibrary.Conv_IntToDouble` SizeY) 1.0)) "Undefined" "OverrideRootScale" null null))
  (bind _output_get (set `self.Arena` _returnvalue))
  (`self.FN_SpawnObstacles` 50)
  ;[0 0 0] Set NavMeshVolume Bounds according to Arena Bounds for the AI
  (`self.FN_SetNavMeshBounds` (`self.GetActorScale3D` _output_get))
  (return))

(fn `FN_SpawnObstacles`
  (params (Amount :type Integer))
  (bind _returnvalue (`KismetMathLibrary.Conv_IntToDouble` (`KismetMathLibrary.RandomIntegerInRange` 1 5)))
  (for _ (range (+ Amount 1))
    (`|SpawnActorFromClass` "/Game/Levels/Game/Prototyping/BP_Obstacle.BP_Obstacle_C" (`KismetMathLibrary.MakeTransform` (`KismetMathLibrary.MakeVector` (`KismetMathLibrary.RandomFloatInRange` -7000.0 7000.0) (`KismetMathLibrary.RandomFloatInRange` -7000.0 7000.0) 20.0) (`KismetMathLibrary.RandomRotator` true) (`KismetMathLibrary.MakeVector` _returnvalue _returnvalue _returnvalue)) "AdjustIfPossibleButAlwaysSpawn" "OverrideRootScale" null null))
  (return))

(fn `FN_SpawnShips`
  (locals (PlayerIndexLocal :type Integer))
  (for _index (range (`KismetArrayLibrary.Array_Length` (`self.PlayerStarts`)))
    (set `local.PlayerIndexLocal` _index)
    (bind _returnvalue (`|SpawnActorFromClass` "/Game/Levels/Game/Characters/Ship/BP_Ship.BP_Ship_C" (`self.GetTransform` (`|GetArrayItem` (`self.PlayerStarts`) _index)) "AdjustIfPossibleButAlwaysSpawn" "OverrideRootScale" null null))
    (set `/Game/Levels/Game/Characters/Ship/BP_Ship.ShipId` (`local.PlayerIndexLocal`) _returnvalue)
    (`KismetArrayLibrary.Array_Add` (`self.ShipArray`) _returnvalue)))

(fn `FN_SpawnStartPosition`
  (returns (StartPosition :type "/Game/Levels/Game/Player/BP_PlayerStart Object Reference"))
  (bind _returnvalue (`|SpawnActorFromClass` "/Game/Levels/Game/Player/BP_PlayerStart.BP_PlayerStart_C" (`KismetMathLibrary.MakeTransform` (`KismetMathLibrary.MakeVector` (`KismetMathLibrary.RandomFloatInRange` -10000.0 10000.0) (`KismetMathLibrary.RandomFloatInRange` -10000.0 10000.0) 500.0)) "AdjustIfPossibleButAlwaysSpawn" "OverrideRootScale" null null))
  (return _returnvalue))

(fn `FN_SpawnStartPositions`
  (params (Amount :type Integer))
  (for _ (range Amount)
    (bind _startposition (`self.FN_SpawnStartPosition`))
    (`KismetArrayLibrary.Array_Add` (`self.PlayerStarts`) _startposition))
  (return))

(fn `UserConstructionScript`)