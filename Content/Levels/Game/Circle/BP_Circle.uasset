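; BP_Circle is an actor that lays out static mesh instances along a procedurally built circular spline.
; On BeginPlay, FNGetRadialPoint uses sine and cosine of evenly stepped angles to place one local-space spline point per segment at the set radius.
; CalculateNumberOfInstances derives a count from spline length and spacing, then the InstancedStaticMesh adds instances at those distances, rotated to follow the spline.
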(event EventBeginPlay
  (bind _spline (Variables|Default|GetSpline))
  (for _index (range 0 (- (Variables|Default|GetSegments) 1))
    (CallFunction|FNGetRadialPoint _index))
  (Components|StaticMesh|SetStaticMesh (Variables|Default|GetInstancedStaticMesh) (Variables|Default|GetStaticMeshVar))
  (for _index_2 (range 0 (Utilities|CalculateNumberOfInstances))
    (Components|InstancedStaticMesh|AddInstance (Variables|Default|GetInstancedStaticMesh) (Math|Transform|MakeTransform (Spline|GetLocationatDistanceAlongSpline _spline (* _index_2 (Variables|Default|GetSpaceBetweenInstances)) "Local") (Spline|GetRotationatDistanceAlongSpline _spline (* _index_2 (Variables|Default|GetSpaceBetweenInstances)) "Local") "1.000000,1.000000,1.000000") false)))

(event Collision|EventActorBeginOverlap
  (params (OtherActor :type Actor%20Object%20Reference)))

(event EventTick
  (params (DeltaSeconds :type Float%20%28single-precision%29)))

(fn ConstructionScript)

(fn FNGetRadialPoint
  (params (Segment :type Integer))
  (bind _returnvalue (Math|Trig|GetPI))
  (bind _returnvalue_2 (Math|Trig|GetPI))
  (bind _radius (Variables|Default|GetRadius))
  (bind _radius_2 (Variables|Default|GetRadius))
  (bind _segments (Variables|Default|GetSegments))
  (bind _returnvalue_3 (/ 360 _segments))
  (bind _returnvalue_4 (* _returnvalue_3 Segment))
  (bind _returnvalue_5 (Math|Conversions|ToFloat(Integer) _returnvalue_4))
  (bind _returnvalue_6 (Math|Conversions|ToFloat(Integer) _returnvalue_4))
  (bind _returnvalue_7 (|(r*(cos((d*((pi*2)/360))))) _radius _returnvalue_5 _returnvalue))
  (bind _returnvalue_8 (|(r*(sin((d*((pi*2)/360))))) _radius_2 _returnvalue_6 _returnvalue_2))
  (bind _returnvalue_9 (Math|Vector2D|MakeVector2D _returnvalue_7 _returnvalue_8))
  (Utilities|FlowControl|Sequence
    (:then_0
      (LocalVariables|SetCenter (Transformation|GetActorLocation)))
    (:then_1
      (if (== Segment 0)
        (Spline|SetLocationatSplinePoint (Variables|Default|GetSpline) 0 (Math|Vector|MakeVector (.x _returnvalue_9) (.y _returnvalue_9) 0.0) "Local" true)
        (else
          (Spline|AddSplinePoint (Variables|Default|GetSpline) (Math|Vector|MakeVector (.x _returnvalue_9) (.y _returnvalue_9) 0.0) "Local" true))))))