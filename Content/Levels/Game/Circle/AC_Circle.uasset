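; Actor component that draws a circle of repeated line meshes on its owner, with events to show, hide or change its radius.
; It adds a closed-loop spline at runtime from trigonometric radial points, then places collision-free instanced static meshes at even spacing along it.
; Hiding clears points and instances.
; Radius changes destroy the spline and rebuild, adding a new instanced mesh component while the old one is only cleared.
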(event Custom|ChangeRadiusEvent
  (params (Radius :type Float%20%28double-precision%29))
  (Circle|Management|FNChangeRadius Radius))

(event Custom|HideCircleEvent
  (Circle|Management|FNHideCircle))

(event Custom|ShowCircleEvent
  (Circle|Management|FNShowCircle))

(fn FNChangeRadius
  (params (Radius :type Float%20%28double-precision%29))
  (Variables|Default|SetRadius Radius)
  (Circle|Management|FNDestroyCircle)
  (Circle|Management|FNCreateCircle)
  (return))

(fn FNCreateCircle
  (Utilities|FlowControl|Sequence
    (:then_0
      (Circle|InstancedStaticMesh|FNCreateInstancedStaticMesh))
    (:then_1
      (Circle|SplineComponent|FNCreateSplineComponent))
    (:then_2
      (Circle|SplinePointsFunctions|FNAddSplinePoints))
    (:then_3
      (Circle|SplinePointsFunctions|FNSetSplinePoints))
    (:then_4
      (Circle|InstancedStaticMesh|FNAddSplineMeshInstance))))

(fn FNGetRadialPoint
  (params (Segment :type Integer))
  (bind _returnvalue (|((360/{99D35565-4BB1-D0F1-E045-CF9C23733ECA})*segment) Segment))
  (return (Math|Vector2D|MakeVector2D (|(r*(cos((d*((pi*2)/360))))) (Variables|Default|GetRadius) (Math|Conversions|ToFloat(Integer) _returnvalue) (Math|Trig|GetPI)) (|(r*(sin((d*((pi*2)/360))))) (Variables|Default|GetRadius) (Math|Conversions|ToFloat(Integer) _returnvalue) (Math|Trig|GetPI)))))

(fn FNClearSplinePoints
  (bind _spline (Variables|Default|GetSpline))
  (Utilities|IsValid _spline
    (:Is%20Valid
      (Spline|ClearSplinePoints _spline true))
    (:Is%20Not%20Valid
      _))
  (return))

(fn FNAddSplinePoints
  (for _index (range 0 (- (Variables|Default|GetSegments) 1))
    (Spline|AddSplinePoint (Variables|Default|GetSpline) (Math|Vector|MakeVector 0.0 0.0 0.0) "Local" true)))

(fn FNSetSplinePoints
  (for _index (range 0 (Variables|Default|GetSegments))
    (Spline|SetLocationatSplinePoint (Variables|Default|GetSpline) _index (Math|Vector|MakeVector (.x (Circle|Math|FNGetRadialPoint _index)) (.y (Circle|Math|FNGetRadialPoint _index)) 0.0) "Local" true)
    (Spline|SetSplinePointType (Variables|Default|GetSpline) _index "Curve" true)))

(fn FNAddSplineMeshInstance
  (Components|StaticMesh|SetStaticMesh (Variables|Default|GetInstancedStaticMesh) (Variables|CircleSettings|GetLineMesh))
  (for _index (range 0 (Utilities|CalculateNumberOfInstances))
    (Components|InstancedStaticMesh|AddInstance (Variables|Default|GetInstancedStaticMesh) (Math|Transform|MakeTransform (Spline|GetLocationatDistanceAlongSpline (Variables|Default|GetSpline) (* _index (Variables|Default|GetSpaceBetweenInstances)) "Local") (Spline|GetRotationatDistanceAlongSpline (Variables|Default|GetSpline) (* _index (Variables|Default|GetSpaceBetweenInstances)) "Local") "1.000000,1.000000,1.000000") false)))

(fn FNCreateSplineComponent
  (bind _returnvalue (Game|AddComponentbyClass (Components|GetOwner) "/Script/Engine.SplineComponent" false))
  (Spline|SetClosedLoop _returnvalue true true)
  (Spline|ClearSplinePoints _returnvalue true)
  (Variables|Default|SetSpline _returnvalue)
  (return))

(fn FNDestroySplineComponent
  (bind _spline (Variables|Default|GetSpline))
  (Utilities|IsValid _spline
    (:Is%20Valid
      (Components|DestroyComponent _spline))
    (:Is%20Not%20Valid
      _))
  (return))

(fn FNCreateInstancedStaticMesh
  (bind _returnvalue (Game|AddComponentbyClass (Components|GetOwner) "/Script/Engine.InstancedStaticMeshComponent" false))
  (Collision|SetCollisionEnabled _returnvalue "NoCollision")
  (Variables|Default|SetInstancedStaticMesh _returnvalue)
  (return))

(fn FNClearInstancedStaticMesh
  (bind _instancedstaticmesh (Variables|Default|GetInstancedStaticMesh))
  (Utilities|IsValid _instancedstaticmesh
    (:Is%20Valid
      (Components|InstancedStaticMesh|ClearInstances _instancedstaticmesh))
    (:Is%20Not%20Valid
      _))
  (return))

(fn FNDestroyCircle
  (Utilities|FlowControl|Sequence
    (:then_0
      (Circle|InstancedStaticMesh|FNClearInstancedStaticMesh))
    (:then_1
      (Circle|SplinePointsFunctions|FNClearSplinePoints))
    (:then_2
      (Circle|SplineComponent|FNDestroySplineComponent))))

(fn FNHideCircle
  (Utilities|FlowControl|Sequence
    (:then_0
      (Circle|InstancedStaticMesh|FNClearInstancedStaticMesh))
    (:then_1
      (Circle|SplinePointsFunctions|FNClearSplinePoints))))

(fn FNShowCircle
  (Utilities|FlowControl|Sequence
    (:then_0
      (Circle|SplinePointsFunctions|FNAddSplinePoints))
    (:then_1
      (Circle|SplinePointsFunctions|FNSetSplinePoints))
    (:then_2
      (Circle|InstancedStaticMesh|FNAddSplineMeshInstance))))