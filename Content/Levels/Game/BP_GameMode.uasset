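; Game mode that tracks joining players and holds match start until the player count equals the maximum.
; PostLogin adds each BP_PlayerController to a list and prints a success message with the player's name.
; The ReadyToStartMatch override compares NumPlayers to MaxPlayers.
; A helper returns the cast BP_GameState, but its only use, a MatchStartedEvent call once the game is full, sits in unwired logic that never runs.
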(event `self.K2_PostLogin`
  (params (NewPlayer :type "PlayerController Object Reference"))
  (bind _asbp_player_controller (cast `/Game/Levels/Game/BP_PlayerController` NewPlayer))
  (`KismetArrayLibrary.Array_Add` (`self.PlayerControllerList`) _asbp_player_controller)
  (`/Game/Libraries/PrintLib.PrintSuccess` (`self.PrintLib`) (`KismetStringLibrary.Concat_StrStr` "added " (`PlayerState.GetPlayerName` (`Controller.PlayerState` _asbp_player_controller)) " to PlayerList!") 20.0))

(fn `FN_GetGameState`
  (returns (GameState :type "/Game/Levels/Game/BP_GameState Object Reference"))
  (bind _asbp_game_state (cast `/Game/Levels/Game/BP_GameState` (`GameplayStatics.GetGameState`)))
  (return _asbp_game_state))

(fn `ReadyToStartMatch`
  (returns (ReturnValue :type Boolean))
  (return (== (`self.NumPlayers`) (`self.MaxPlayers`))))

(fn `UserConstructionScript`)