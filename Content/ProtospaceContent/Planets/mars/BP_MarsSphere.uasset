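; BP_MarsSphere is a Mars planet sphere that orients the night side of its material relative to a referenced Sun actor.
; FNSetNightSideDirection computes the normalized direction from PlanetMesh toward the Sun and writes it to the LightDirection vector parameter on the mesh's materials.
; It runs in the Construction Script and on BeginPlay, with no per-frame update.
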(event `self.ReceiveBeginPlay`
  (`self.FN_SetNightSideDirection`))

(event `self.ReceiveTick`
  (params (DeltaSeconds :type "Float (single-precision)")))

(fn `FN_SetNightSideDirection`
  (`MeshComponent.SetVectorParameterValueOnMaterials` (`self.PlanetMesh`) "LightDirection" (* (`KismetMathLibrary.GetForwardVector` (`KismetMathLibrary.FindLookAtRotation` (`self.K2_GetActorLocation` (`self.Sun`)) (`SceneComponent.K2_GetComponentLocation` (`self.PlanetMesh`)))) (-1.0 -1.0 -1.0))))

(fn `UserConstructionScript`
  (`self.FN_SetNightSideDirection`))