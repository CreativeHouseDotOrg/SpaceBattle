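; BP_MusicPlayer is a music player actor that plays tracks from MusicList through a Media Player and media sound component, which stays tickable while paused.
; BeginPlay initializes the player and binds media delegates through collapsed graphs with debug prints.
; OpenSourceEvent loads a track by index, opening triggers Play, and reaching the end reopens the first track.
; DoOnce gates on resume, suspend and end callbacks re-arm whenever playback starts.
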(event `OnMediaOpenedBindEvent`
  (params (OpenedUrl :type String))
  (`KismetSystemLibrary.PrintString` (`KismetStringLibrary.Concat_StrStr` "Play  " OpenedUrl) true true (struct :`G` 1.0 :`B` 0.064089 :`A` 1.0) 5.0)
  (`self.OnMediaOpenedEvent`))

(event `OnPlaybackSuspendedEvent`)

(event `OnMediaOpenFailed_Event`
  (params (FailedUrl :type String))
  (`KismetSystemLibrary.PrintString` (`KismetStringLibrary.Concat_StrStr` "Play failed " FailedUrl) true true (struct :`R` 1.0 :`B` 0.008376 :`A` 1.0) 5.0))

(event `self.ReceiveBeginPlay`
  (`self.FN_InitMusicPlayer`)
  (`|ExecutionSequence`
    (:`then_0`
      (add `MediaPlayer.OnMediaOpened` (`self.MediaPlayer`) (delegate `OnMediaOpenedBindEvent`)))
    (:`then_1`
      (add `MediaPlayer.OnMediaOpenFailed` (`self.MediaPlayer`) (delegate `OnMediaOpenFailed_Event`)))
    (:`then_2`
      (add `MediaPlayer.OnPlaybackResumed` (`self.MediaPlayer`) (delegate `OnPlaybackResumedBindEvent`)))
    (:`then_3`
      (add `MediaPlayer.OnPlaybackSuspended` (`self.MediaPlayer`) (delegate `OnPlaybackSuspendedBindEvent`)))
    (:`then_4`
      (add `MediaPlayer.OnEndReached` (`self.MediaPlayer`) (delegate `OnEndReachedBindEvent`)))))

(event `OnPlaybackResumedBindEvent`
  (`/Engine/EditorBlueprintResources/StandardMacros.DoOnce` false :!label _label
    (:`Completed`
      (`KismetSystemLibrary.PrintString` "Playback Resumed" true true (struct :`R` 1.0 :`G` 0.926622 :`A` 1.0) 5.0)
      (`self.OnPlaybackResumedEvent`))))

(event `OnPlaybackResumedEvent`)

(event `OnPlaybackSuspendedBindEvent`
  (`/Engine/EditorBlueprintResources/StandardMacros.DoOnce` false :!label _label_2
    (:`Completed`
      (`KismetSystemLibrary.PrintString` "Playback suspended" true true (struct :`R` 1.0 :`G` 0.402985 :`A` 1.0) 5.0)
      (`self.OnPlaybackSuspendedEvent`))))

(event `OnMediaOpenedEvent`
  ;[0 0 0] Play Music
  (`self.PlayEvent`)
  (`|ExecutionSequence` :!label _label_3
    (:`then_0`
      (goto _label :!via `Reset`))
    (:`then_1`
      (goto _label_2 :!via `Reset`))
    (:`then_2`
      (goto _label_4 :!via `Reset`))))

(event `OnEndReachedEvent`
  (bind _output_get (set `self.CurrentMediaIndex` 0))
  (`self.OpenSourceEvent` _output_get))

(event `OnEndReachedBindEvent`
  (`/Engine/EditorBlueprintResources/StandardMacros.DoOnce` false :!label _label_4
    (:`Completed`
      (`KismetSystemLibrary.PrintString` "End Reached!" true true (struct :`R` 1.0 :`G` 0.125939 :`A` 1.0) 5.0)
      (`self.OnEndReachedEvent`))))

(event `OpenSourceEvent`
  (params (Index :type Integer))
  (`self.FN_OpenSource` Index))

(event `PlayEvent`
  (`MediaPlayer.Play` (`self.MediaPlayer`))
  (goto _label_3))

(event `PauseEvent`
  (`MediaPlayer.Pause` (`self.MediaPlayer`)))

(fn `FN_InitMusicPlayer`
  (returns (MusicPlayer :type "MediaPlayer Object Reference"))
  (bind _msc_musicplayer (`self.MSC_MusicPlayer`))
  (`MediaSoundComponent.SetMediaPlayer` _msc_musicplayer "/Game/Music/MP_MusicPlayer.MP_MusicPlayer")
  (`ActorComponent.SetTickableWhenPaused` _msc_musicplayer true)
  (bind _output_get (set `self.MediaPlayer` (`MediaSoundComponent.GetMediaPlayer` (`self.MSC_MusicPlayer`))))
  (return _output_get))

(fn `FN_OpenSource`
  (params (CurrentMediaIndex :type Integer))
  (bind _output_get (set `self.CurrentMediaIndex` CurrentMediaIndex))
  (`MediaPlayer.OpenSource` (`self.MediaPlayer`) (`|GetArrayItem` (`self.MusicList`) _output_get)))

(fn `GetCurrentMusicTrack`
  (returns (MediaSource :type "MediaSource Object Reference"))
  (return (`|GetArrayItem` (`self.MusicList`) (`self.CurrentMediaIndex`))))

(fn `UserConstructionScript`)